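; BP_VoidCharacter is a character Blueprint that adds a dash camera effect and sword spawning.
; SetCameraFov captures the follow camera's current FOV, blends it to the dash FOV on one timeline, then chains a second timeline with its own alpha curve.
; Pressing E spawns a BP_Sword and snaps it to the mesh's SwordSocket, with no check for an existing sword.
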(event EventBeginPlay)

(event Collision|EventActorBeginOverlap
  (params (OtherActor :type Actor%20Object%20Reference)))

(event EventTick
  (params (DeltaSeconds :type Float%20%28single-precision%29)))

(event EventSetCameraFov
  ;[1 1 1] Change Camera FOV on Dash
  (Variables|Default|SetCamDefaultFov (Variables|/Script/Engine.CameraComponent|GetFieldOfView (Variables|Default|GetFollowCamera)))
  (bind _cameralerp (Timeline|Timeline Play)
    (:Update
      (Camera|SetFieldOfView (Variables|Default|GetFollowCamera) (Math|Float|Lerp (Variables|Default|GetCamDefaultFov) (Variables|Default|GetCamDashFov) _cameralerp)))
    (:Finished
      (bind _camfovrev (Timeline|Timeline_0 PlayFromStart)
        (:Update
          (Camera|SetFieldOfView (Variables|Default|GetFollowCamera) (Math|Float|Lerp (Variables|Default|GetCamDefaultFov) (Variables|Default|GetCamDashFov) _camfovrev)))))))

(event Input|KeyboardEvents|E
  (params (Key :type Key%20Structure :default "None"))
  (bind _mesh (Variables|Character|GetMesh))
  (:Pressed
    (bind _returnvalue (Game|SpawnActorfromClass "/Game/_Game/Blueprints/Weapons/Swords/BP_Sword.BP_Sword_C" (Math|Transform|MakeTransform (Transformation|GetSocketLocation _mesh "SwordSocket") (Transformation|GetSocketRotation _mesh "SwordSocket") "1.000000,1.000000,1.000000") "AdjustIfPossibleButAlwaysSpawn" 0 0))
    (Transformation|AttachComponentToComponent _returnvalue (Variables|Character|GetMesh) "SwordSocket" "SnapToTarget" "SnapToTarget" "KeepRelative" true)))

(fn ConstructionScript)